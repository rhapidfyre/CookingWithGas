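; Gameplay ability that lets the player aim a grenade along a previewed arc while input is held and throw it on release.
; A short repeating delay task re-runs TracePath, which predicts the projectile path from the character's firing point.
; BP_FiringArc markers are reused along that path, spawning more as needed and hiding extras.
; Release spawns BP_Grenade at the firing point and ends the ability, destroying the markers.
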(event `self.K2_ActivateAbility`
  (bind _asbp_character_player (cast `/Game/CookingWithGas/Blueprints/BP_Character_Player` (`self.GetAvatarActorFromActorInfo`))
    (:`then`
      (set `self.CharReference` _asbp_character_player)
      (`self.K2_CommitAbility`)
      (`self.TracePath`)
      (`AbilityTask_WaitInputRelease.WaitInputRelease` false
        (:`then`
          (`GameplayTask_WaitDelay.TaskWaitDelay` null 0.001 :!label _label
            (:`OnFinish`
              (`self.TracePath`)
              (goto _label))))
        (:`OnRelease`
          (`self.Fire`)
          (`self.K2_EndAbility`))))
    (:`CastFailed`
      (`self.K2_EndAbility`))))

(event `self.K2_OnEndAbility`
  (params (bWasCancelled :type Boolean))
  (for _array_element (`self.FiringArc`)
    (`Actor.K2_DestroyActor` _array_element)))

(fn `Fire`
  (bind _charreference (`self.CharReference`))
  (bind (_rotation _location) (`/Game/CookingWithGas/Blueprints/BP_Character_Player.CalcFiringPoint` _charreference))
  (`|SpawnActorFromClass` "/Game/CookingWithGas/Blueprints/BP_Grenade.BP_Grenade_C" (`KismetMathLibrary.MakeTransform` _location _rotation) "AlwaysSpawn" "MultiplyWithRoot" _charreference null))

(fn `TracePath`
  (locals (tPathLocations :type "Array of Vector Structure") (tIndex :type Integer))
  (bind _tindex (`local.tIndex`))
  (bind _firingarc (`self.FiringArc`))
  (bind (_rotation _location) (`/Game/CookingWithGas/Blueprints/BP_Character_Player.CalcFiringPoint` (`self.CharReference`)))
  (bind _output (`|GetArrayItem` _firingarc _tindex))
  (`self.CharReference`
    (:`then`
      (`|ExecutionSequence`
        (:`then_0`
          (for _array_element (`self.FiringArc`)
            (`SceneComponent.SetVisibility` (`/Game/CookingWithGas/Blueprints/BP_FiringArc.Sphere` _array_element) false false)))
        (:`then_1`
          (bind (_outhit _outpathpositions) (`GameplayStatics.Blueprint_PredictProjectilePath_ByTraceChannel` _location (* (`KismetMathLibrary.GetForwardVector` _rotation) 2000.0) true 6.0 "ECC_GameTraceChannel1" false (`|MakeArray` (`self.CharReference`) :!type "Actor Object Reference")))
          (bind _output_get (set `local.tPathLocations` _outpathpositions))
          (for _index (range (`KismetMathLibrary.Max` (`KismetArrayLibrary.Array_Length` _output_get) (`KismetArrayLibrary.Array_Length` (`self.FiringArc`))))
            (set `local.tIndex` _index)
            (if (not (`KismetArrayLibrary.Array_IsValidIndex` (`local.tPathLocations`) (`local.tIndex`)))
              (break)
              (elif (`KismetArrayLibrary.Array_IsValidIndex` _firingarc _tindex)
                (`SceneComponent.SetVisibility` (`/Game/CookingWithGas/Blueprints/BP_FiringArc.Sphere` _output) true false)
                (`Actor.K2_SetActorLocation` _output (`|GetArrayItem` (`local.tPathLocations`) (`local.tIndex`)) false true)
                (else
                  (bind _returnvalue (`|SpawnActorFromClass` "/Game/CookingWithGas/Blueprints/BP_FiringArc.BP_FiringArc_C" (`KismetMathLibrary.MakeTransform` (0.0 0.0 0.0)) "AlwaysSpawn" "MultiplyWithRoot" null 0.5 false null))
                  (`KismetArrayLibrary.Array_Add` (`self.FiringArc`) _returnvalue))))))))
    (:`else`)))