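; Gameplay ability that sets off a short series of fiery explosions on a target actor.
; Once committed, it waits for one Event.SetUsUpTheBomb event, then explodes at the payload target's current location four times, a second apart, before ending.
; Each explosion draws a debug sphere and applies GE_Damage, with SetByCaller magnitude and fire tag, to overlapped actors with an Ability System Component.
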(event `self.K2_ActivateAbility`
  (`self.K2_CommitAbility`)
  (bind (_asynctaskproxy _payload) (`AbilityTask_WaitGameplayEvent.WaitGameplayEvent` (struct :`TagName` "Event.SetUsUpTheBomb") null true)
    (:`EventReceived`
      (set `self.Count` 4)
      (if (> (`self.Count`) 0) :!label _label
        (`self.Explode` (`Actor.K2_GetActorLocation` (`.Target` (break `GameplayEventData` _payload))))
        (`/Engine/EditorBlueprintResources/StandardMacros.DecrementInt` (`self.Count`)
          (:`  `
            (`GameplayTask_WaitDelay.TaskWaitDelay` null 1.0
              (:`OnFinish`
                (goto _label)))))
        (else
          (`self.K2_EndAbility`))))))

(fn `Explode`
  (params (Location :type "Vector Structure"))
  (bind _returnvalue (`AbilitySystemBlueprintLibrary.GetAbilitySystemComponent` (`self.GetAvatarActorFromActorInfo`)))
  (`KismetSystemLibrary.DrawDebugSphere` Location 128.0)
  (bind _outactors (`KismetSystemLibrary.SphereOverlapActors` Location 128.0 (`|MakeArray` "ObjectTypeQuery3" "ObjectTypeQuery6" "ObjectTypeQuery4" :!type "EObjectTypeQuery Enum")))
  (for _array_element _outactors
    (bind _returnvalue_2 (`AbilitySystemBlueprintLibrary.GetAbilitySystemComponent` _array_element))
    (`/Engine/EditorBlueprintResources/StandardMacros.IsValid` _returnvalue_2
      (:`Is Valid`
        (bind _returnvalue_3 (`AbilitySystemBlueprintLibrary.AssignTagSetByCallerMagnitude` (`AbilitySystemComponent.MakeOutgoingSpec` :`self` _returnvalue :`GameplayEffectClass` "/Game/CookingWithGas/Effects/Damage/GE_Damage.GE_Damage_C") (struct :`TagName` "Damage.SetByCaller") 5.0))
        (bind _returnvalue_4 (`AbilitySystemBlueprintLibrary.AddAssetTag` _returnvalue_3 (struct :`TagName` "Damage.Type.Fire")))
        (`AbilitySystemComponent.BP_ApplyGameplayEffectSpecToTarget` _returnvalue _returnvalue_4 _returnvalue_2)))))