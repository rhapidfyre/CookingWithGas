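; Gameplay ability that fires projectiles from the player's camera view, either single-shot or full-auto.
; Full-auto repeats at AttacksPerSecond, recommitting before each shot, until input release or a failed commit.
; Each shot passes the projectile an effect spec with SetByCaller damage and a damage-type tag.
; Projectiles spawn along the camera's forward vector, offset by the boom's arm length to cancel the third-person camera distance.
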(event `self.K2_ActivateAbility`
  (if (<= (`self.AttacksPerSecond`) 0.0)
    (set `self.AttacksPerSecond` 1.0))
  (bind _asbp_character_player (cast `/Game/CookingWithGas/Blueprints/BP_Character_Player` (`self.GetAvatarActorFromActorInfo`))
    (:`then`
      (set `self.CharacterReference` _asbp_character_player)
      (`self.K2_CommitAbility`)
      (`self.Fire`)
      ;[0.1 0.1 0.1 0.4] Repeat the projectile if it is a full auto ability
      (if (`self.IsFullAuto`)
        (`AbilityTask_WaitInputRelease.WaitInputRelease` false
          (:`then`
            (`GameplayTask_WaitDelay.TaskWaitDelay` null (/ 1.0 (`self.AttacksPerSecond`)) :!label _label
              (:`OnFinish`
                (bind _returnvalue (`self.K2_CommitAbility`))
                (if _returnvalue
                  (`self.Fire`)
                  (goto _label)
                  (else
                    (`self.K2_EndAbility`))))))
          (:`OnRelease`
            (`self.K2_EndAbility`)))
        (else
          (`self.K2_EndAbility`))))
    (:`CastFailed`
      (`self.K2_EndAbility`))))

(fn `Fire`
  (locals (tFwdVector :type "Vector Structure" :default (0.0 0.0 0.0)) (tWorldRot :type "Rotator Structure" :default (struct)))
  (bind _output_get (set `local.tWorldRot` (`SceneComponent.K2_GetComponentRotation` (`CookingWithGasCharacter.FollowCamera` (`self.CharacterReference`)))))
  (bind _output_get_2 (set `local.tFwdVector` (`KismetMathLibrary.GetForwardVector` _output_get)))
  (bind _spechandle (`self.MakeSpec`))
  (`|SpawnActorFromClass` (`self.ProjectileClass`) (`KismetMathLibrary.MakeTransform` (+ (* _output_get_2 (`SpringArmComponent.TargetArmLength` (`CookingWithGasCharacter.CameraBoom` (`self.CharacterReference`)))) (`SceneComponent.K2_GetComponentLocation` (`CookingWithGasCharacter.FollowCamera` (`self.CharacterReference`)))) (`local.tWorldRot`) (0.4 0.4 0.4)) "AlwaysSpawn" "MultiplyWithRoot" (`self.CharacterReference`) _spechandle null))

(fn `MakeSpec`
  (returns (SpecHandle :type "GameplayEffectSpecHandle Structure"))
  (bind _characterreference (`self.CharacterReference`)
    (:`then`
      (bind _returnvalue (`AbilitySystemBlueprintLibrary.GetAbilitySystemComponent` _characterreference))
      (bind _returnvalue_2 (`AbilitySystemBlueprintLibrary.AssignTagSetByCallerMagnitude` (`AbilitySystemComponent.MakeOutgoingSpec` _returnvalue (`self.GameplayEffectClass`) 0.0 (`AbilitySystemComponent.MakeEffectContext` _returnvalue)) (struct :`TagName` "Damage.SetByCaller") (`self.DamageValue`)))
      (bind _returnvalue_3 (`AbilitySystemBlueprintLibrary.AddAssetTag` _returnvalue_2 (`self.DamageTag`)))
      (return _returnvalue_3))
    (:`else`)))