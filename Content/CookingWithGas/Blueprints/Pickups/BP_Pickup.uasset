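; BP_Pickup is a pickup actor that grants a Gameplay Ability System effect to whatever overlaps it.
; On overlap, it applies EffectClass to the other actor's Ability System Component and destroys itself, ignoring actors without a valid component.
; The construction script gives the Sphere a dynamic instance of GasMaterial tinted by EffectColor, so each pickup's effect and color come from variables.
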(event `self.ReceiveBeginPlay`)

(event `self.ReceiveActorBeginOverlap`
  (params (OtherActor :type "Actor Object Reference"))
  (bind _returnvalue (`AbilitySystemBlueprintLibrary.GetAbilitySystemComponent` OtherActor))
  (`/Engine/EditorBlueprintResources/StandardMacros.IsValid` _returnvalue
    (:`Is Valid`
      (`AbilitySystemComponent.BP_ApplyGameplayEffectToSelf` :`self` _returnvalue :`GameplayEffectClass` (`self.EffectClass`))
      (`self.K2_DestroyActor`))))

(fn `UserConstructionScript`
  (`parent.UserConstructionScript`)
  (bind _returnvalue (`PrimitiveComponent.CreateDynamicMaterialInstance` (`self.Sphere`) 0 (`self.GasMaterial`) "None"))
  (bind _output_get (set `self.DynMaterialInstance` _returnvalue))
  (`MaterialInstanceDynamic.SetVectorParameterValue` _output_get "Color" (`self.EffectColor`)))