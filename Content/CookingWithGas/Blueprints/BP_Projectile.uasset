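; BP_Projectile is a projectile that delivers a Gameplay Ability System effect to whatever it hits, ignoring its owner.
; On Hit, if both owner and hit actor have ability system components, it adds the hit result to the SpecHandle's effect context and applies the spec from owner to target.
; It then destroys itself after any non-owner hit, even when no effect applies.
; A debug function that prints the hit component and bone is left unconnected.
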(event `self.ReceiveHit`
  (params (MyComp :type "PrimitiveComponent Object Reference") (Other :type "Actor Object Reference") (OtherComp :type "PrimitiveComponent Object Reference") (bSelfMoved :type Boolean) (HitLocation :type "Vector Structure") (HitNormal :type "Vector Structure") (NormalImpulse :type "Vector Structure") (Hit :type "HitResult Structure (by ref)"))
  (bind _returnvalue (`AbilitySystemBlueprintLibrary.GetAbilitySystemComponent` Other))
  (bind _returnvalue_2 (`AbilitySystemBlueprintLibrary.GetAbilitySystemComponent` (`self.GetOwner`)))
  (if (!= Other (`self.GetOwner`))
    (`|ExecutionSequence`
      (:`then_0`
        (`/Engine/EditorBlueprintResources/StandardMacros.IsValid` _returnvalue_2
          (:`Is Valid`
            (`/Engine/EditorBlueprintResources/StandardMacros.IsValid` _returnvalue
              (:`Is Valid`
                (bind _returnvalue_3 (`AbilitySystemBlueprintLibrary.GetEffectContext` (`self.SpecHandle`)))
                (`AbilitySystemBlueprintLibrary.EffectContextAddHitResult` _returnvalue_3 Hit)
                (`AbilitySystemComponent.BP_ApplyGameplayEffectSpecToTarget` _returnvalue_2 (`self.SpecHandle`) _returnvalue))))))
      (:`then_1`
        (`self.K2_DestroyActor`)))))

(fn `PrintHitData`
  (params (OtherComp :type "Object Object Reference") (Hit :type "HitResult Structure (by ref)"))
  (`KismetSystemLibrary.PrintString` (`KismetStringLibrary.Concat_StrStr` (`KismetSystemLibrary.GetDisplayName` OtherComp) ", " (`KismetStringLibrary.Conv_NameToString` (`.HitBoneName` (`GameplayStatics.BreakHitResult` Hit))))))

(fn `UserConstructionScript`)