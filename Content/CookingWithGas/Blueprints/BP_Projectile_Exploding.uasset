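; BP_Projectile_Exploding is a projectile that triggers the GA_Exploding gameplay ability when it hits an actor that has an Ability System Component.
; On such a hit, it grants and activates the ability once on its owner's Ability System Component.
; It then sends the owner an Event.SetUsUpTheBomb gameplay event, with the owner as instigator and the hit actor as target, and destroys itself.
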(event `self.ReceiveHit`
  (params (MyComp :type "PrimitiveComponent Object Reference") (Other :type "Actor Object Reference") (OtherComp :type "PrimitiveComponent Object Reference") (bSelfMoved :type Boolean) (HitLocation :type "Vector Structure") (HitNormal :type "Vector Structure") (NormalImpulse :type "Vector Structure") (Hit :type "HitResult Structure (by ref)"))
  (bind _returnvalue (`self.GetOwner`))
  (bind _returnvalue_2 (`AbilitySystemBlueprintLibrary.GetAbilitySystemComponent` _returnvalue))
  (`/Engine/EditorBlueprintResources/StandardMacros.IsValid` (`AbilitySystemBlueprintLibrary.GetAbilitySystemComponent` Other)
    (:`Is Valid`
      (`/Engine/EditorBlueprintResources/StandardMacros.IsValid` _returnvalue_2
        (:`Is Valid`
          (`AbilitySystemComponent.K2_GiveAbilityAndActivateOnce` _returnvalue_2 "/Game/CookingWithGas/Abilities/GA_Exploding.GA_Exploding_C" 0 -1)
          (`AbilitySystemBlueprintLibrary.SendGameplayEventToActor` _returnvalue (struct :`TagName` "Event.SetUsUpTheBomb") (make `GameplayEventData` (struct) _returnvalue Other))
          (`self.K2_DestroyActor`))))))

(fn `UserConstructionScript`
  (`parent.UserConstructionScript`))