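; BP_Character_Enemy is an enemy character built on the Gameplay Ability System that jumps every tick and reacts to attribute changes.
; On BeginPlay it binds its overhead widget to itself.
; Rising Chilled slows it through CustomTimeDilation; at the maximum, it stops its time completely and applies GE_Debuff_Freeze.
; Health and armor changes, death and armor depletion only print debug messages.
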(event `self.ReceiveTick`
  (params (DeltaSeconds :type "Float (single-precision)"))
  (`self.Jump`))

(event `self.ReceiveBeginPlay`
  (bind _aswbp_character_overhead (cast `/Game/CookingWithGas/Widgets/WBP_Character_Overhead` (`WidgetComponent.GetWidget` (`self.Widget`))))
  (`/Game/CookingWithGas/Widgets/WBP_Character_Overhead.InitCharacter` _aswbp_character_overhead self))

(event `self.OnHealthChanged`
  (params (OldValue :type "Float (single-precision)") (NewValue :type "Float (single-precision)"))
  (`KismetSystemLibrary.PrintString` (`KismetStringLibrary.Concat_StrStr` "Health Modified... " (`KismetStringLibrary.Conv_DoubleToString` NewValue) ",  (" (`KismetStringLibrary.Conv_DoubleToString` (- NewValue OldValue)) ")") true true (struct :`G` 0.66 :`B` 1.0 :`A` 1.0) 5.0))

(event `self.OnArmorChanged`
  (params (OldValue :type "Float (single-precision)") (NewValue :type "Float (single-precision)"))
  (`KismetSystemLibrary.PrintString` (`KismetStringLibrary.Concat_StrStr` "Armor Modified... " (`KismetStringLibrary.Conv_DoubleToString` NewValue) ", (" (`KismetStringLibrary.Conv_DoubleToString` (- NewValue OldValue)) ")") true true (struct :`G` 0.66 :`B` 1.0 :`A` 1.0) 5.0))

(event `self.OnOutOfHealth`
  (params (DamageInstigator :type "Actor Object Reference") (DamageCauser :type "Actor Object Reference") (DamageSpec :type "GameplayEffectSpec Structure (by ref)") (DamageMagnitude :type "Float (single-precision)"))
  (`KismetSystemLibrary.PrintString` "Dead"))

(event `self.OnChilledChanged`
  (params (OldValue :type "Float (single-precision)") (NewValue :type "Float (single-precision)"))
  (set `self.CustomTimeDilation` (`KismetMathLibrary.MapRangeClamped` NewValue 0.0 100.0 1.0 0.5))
  (if (>= NewValue 100.0)
    (set `self.CustomTimeDilation` 0.0)
    (`AbilitySystemComponent.BP_ApplyGameplayEffectToSelf` :`self` (`self.AbilitySystemComponent`) :`GameplayEffectClass` "/Game/CookingWithGas/Effects/Debuffs/GE_Debuff_Freeze.GE_Debuff_Freeze_C")))

(event `self.OnOutOfArmor`
  (params (DamageInstigator :type "Actor Object Reference") (DamageCauser :type "Actor Object Reference") (DamageSpec :type "GameplayEffectSpec Structure (by ref)") (DamageMagnitude :type "Float (single-precision)"))
  (`KismetSystemLibrary.PrintString` "Armor Depleted"))

(fn `UserConstructionScript`)