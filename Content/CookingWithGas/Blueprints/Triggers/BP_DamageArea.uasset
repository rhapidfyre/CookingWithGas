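; Trigger area actor that deals periodic damage to pawns and destructibles inside its box.
; A looping timer started on BeginPlay runs a box overlap query at each DamagePeriod, using the Box component's location and extent.
; Each overlapped actor with an Ability System Component applies a GE_Damage spec to itself, with DamageDealt passed as a SetByCaller magnitude.
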(event `self.ReceiveBeginPlay`
  (`KismetSystemLibrary.K2_SetTimerDelegate` (`|CreateDelegate` :!event `Callback_DamageTimer`) (`KismetMathLibrary.FClamp` (`self.DamagePeriod`) 0.01 1000000.0) true))

(event `Callback_DamageTimer`
  (bind _box (`self.Box`))
  (bind _outactors (`KismetSystemLibrary.BoxOverlapActors` (`SceneComponent.K2_GetComponentLocation` _box) (`BoxComponent.BoxExtent` _box) (`|MakeArray` "ObjectTypeQuery3" "ObjectTypeQuery6" :!type "EObjectTypeQuery Enum")))
  (for _array_element _outactors
    (bind _returnvalue (`AbilitySystemBlueprintLibrary.GetAbilitySystemComponent` _array_element))
    (`/Engine/EditorBlueprintResources/StandardMacros.IsValid` _returnvalue
      (:`Is Valid`
        (bind _returnvalue_2 (`AbilitySystemBlueprintLibrary.AssignTagSetByCallerMagnitude` (`AbilitySystemComponent.MakeOutgoingSpec` _returnvalue "/Game/CookingWithGas/Effects/Damage/GE_Damage.GE_Damage_C" 0.0 (`AbilitySystemComponent.MakeEffectContext` _returnvalue)) (struct :`TagName` "Damage.SetByCaller") (`self.DamageDealt`)))
        (`AbilitySystemComponent.BP_ApplyGameplayEffectSpecToSelf` _returnvalue _returnvalue_2)))))

(fn `UserConstructionScript`)