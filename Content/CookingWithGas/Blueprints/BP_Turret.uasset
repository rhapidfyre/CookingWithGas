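; BP_Turret is a turret that repeatedly fires projectiles at the player character.
; On BeginPlay it starts a looping timer whose interval is randomized once per turret.
; Each shot spawns a BP_Projectile from above its Arrow component, aimed at a raised point on the player.
; It passes the projectile a GE_Damage spec from its own Ability System Component, with damage set through a SetByCaller tag.
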(event `self.ReceiveBeginPlay`
  (`KismetSystemLibrary.K2_SetTimerDelegate` (delegate `FireProjectile`) (`KismetMathLibrary.RandomFloatInRange` 1.6 3.0) true))

(event `FireProjectile`
  (bind _returnvalue (`AbilitySystemBlueprintLibrary.GetAbilitySystemComponent` null))
  (bind _returnvalue_2 (+ (`SceneComponent.K2_GetComponentLocation` (`self.Arrow`)) (0.0 0.0 100.0)))
  (bind _returnvalue_3 (`AbilitySystemBlueprintLibrary.AssignTagSetByCallerMagnitude` (`AbilitySystemComponent.MakeOutgoingSpec` _returnvalue "/Game/CookingWithGas/Effects/Damage/GE_Damage.GE_Damage_C" 0.0 (`AbilitySystemComponent.MakeEffectContext` _returnvalue)) (struct :`TagName` "Damage.SetByCaller") 1.0))
  (`|SpawnActorFromClass` "/Game/CookingWithGas/Blueprints/BP_Projectile.BP_Projectile_C" (`KismetMathLibrary.MakeTransform` _returnvalue_2 (`KismetMathLibrary.Conv_VectorToRotator` (- (+ (`self.K2_GetActorLocation` (`GameplayStatics.GetPlayerCharacter` 0)) (0.0 0.0 90.0)) _returnvalue_2))) "AlwaysSpawn" "MultiplyWithRoot" self _returnvalue_3 null))

(fn `UserConstructionScript`)