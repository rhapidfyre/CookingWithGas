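; Floating text actor that shows a damage icon and colored text through a widget component.
; On BeginPlay it casts the component's widget to WBP_FloatingText, then applies the DamageIcon texture, DamageText and DamageColor to its image and text elements.
; The blueprint only sets the initial content; its graphs contain no movement or lifetime logic.
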(event `self.ReceiveBeginPlay`
  (bind _aswbp_floating_text (cast `/Game/CookingWithGas/Effects/WBP_FloatingText` (`WidgetComponent.GetUserWidgetObject` (`self.Widget`))))
  (`|ExecutionSequence`
    (:`then_0`
      (`Image.SetBrushFromTexture` (`/Game/CookingWithGas/Effects/WBP_FloatingText.Image_FloatingText` _aswbp_floating_text) (`self.DamageIcon`) false))
    (:`then_1`
      (bind _text_floatingtext (`/Game/CookingWithGas/Effects/WBP_FloatingText.Text_FloatingText` _aswbp_floating_text))
      (`TextBlock.SetText` _text_floatingtext (`self.DamageText`))
      (`TextBlock.SetColorAndOpacity` _text_floatingtext (make `SlateColor` (`self.DamageColor`))))))

(fn `UserConstructionScript`)