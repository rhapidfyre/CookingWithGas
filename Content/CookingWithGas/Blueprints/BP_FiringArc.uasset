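; BP_FiringArc is a firing-arc Blueprint with an optional directional arrow that flashes between red and white.
; BeginPlay uses ShowDirectional to control both the arrow's visibility and whether the actor ticks.
; Tick wraps a time value over twice LengthOfFlash and turns it into a triangle wave driving the semi-transparent arrow's green and blue channels.
; An ArrowFlash timeline loop remains in the graph but never runs.
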(event `self.ReceiveBeginPlay`
  (bind _bshowdirectional (`self.bShowDirectional`))
  (`self.SetActorTickEnabled` _bshowdirectional)
  (`SceneComponent.SetHiddenInGame` (`self.Arrow`) (not _bshowdirectional) false))

(event `self.ReceiveTick`
  (params (DeltaSeconds :type "Float (single-precision)"))
  (bind _returnvalue (mod (`self.Delta Seconds`) (`self.Length of Flash`)))
  (bind _returnvalue_2 (/ (`KismetMathLibrary.SelectFloat` (- (`self.Length of Flash`) _returnvalue) _returnvalue (> (/ (`self.Delta Seconds`) (`self.Length of Flash`)) 1.0)) (`self.Length of Flash`)))
  (set `self.Delta Seconds` (mod (+ DeltaSeconds (`self.Delta Seconds`)) (* (`self.Length of Flash`) 2.0)))
  (`ArrowComponent.SetArrowColor` (`self.Arrow`) (`KismetMathLibrary.MakeColor` 1.0 _returnvalue_2 _returnvalue_2 0.5)))

(fn `UserConstructionScript`)